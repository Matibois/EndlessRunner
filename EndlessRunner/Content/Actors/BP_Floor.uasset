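; BP_Floor is a floor segment, apparently for a runner game, that places its own random obstacle and signals when the runner reaches its trigger.
; On BeginPlay it spawns a random class from Obstacles at a random point in a flat area around Extent, storing it as CreatedObstacle.
; Box overlap by BP_RunCharacter binds an empty handler to the Exited dispatcher, then broadcasts it with itself.
; GetAttachTransform exposes AttachPoint's world transform.
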(event `self.ReceiveBeginPlay`
  (`self.SpawnObstacle`))

(event `self.Box.OnComponentBeginOverlap`
  (params (OverlappedComponent :type "PrimitiveComponent Object Reference") (OtherActor :type "Actor Object Reference") (OtherComp :type "PrimitiveComponent Object Reference") (OtherBodyIndex :type Integer) (bFromSweep :type Boolean) (SweepResult :type "HitResult Structure (by ref)"))
  (cast `/Game/Actors/BP_RunCharacter` OtherActor)
  (add `self.Exited` (delegate `Exited_Event`))
  (`self.Exited` self))

(event `Exited_Event` :!signature `self.Exited`
  (params (NewParam :type "/Game/Actors/BP_Floor Object Reference")))

(fn `GetAttachTransform`
  (returns (OutTransform :type "Transform Structure"))
  (return (`SceneComponent.K2_GetComponentToWorld` (`self.Attach point`))))

(fn `SpawnObstacle`
  (bind _returnvalue (`|SpawnActorFromClass` (`KismetArrayLibrary.Array_Random` (`self.Obstacles`)) (`KismetMathLibrary.Conv_VectorToTransform` (`KismetMathLibrary.RandomPointInBoundingBox` (`SceneComponent.K2_GetComponentLocation` (`self.Extent`)) (250.0 250.0 0.0))) "Undefined" "MultiplyWithRoot" null null))
  (set `self.CreatedObstacle` _returnvalue))

(fn `UserConstructionScript`)